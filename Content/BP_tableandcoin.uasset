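; Table-and-coin actor that runs a one-time physical coin flip to set the Player boolean in GI_mainmenu.
; The flip event launches the mesh with randomized vertical and angular impulses, and a flag blocks repeat flips.
; Tick checks whether Head or Tail overlaps Plane, writing true for Head and false for Tail, with DoOnce gates re-armed when contact ends.
; Input is enabled shortly after BeginPlay.
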(event Custom|flip
  (bind _staticmesh (Variables|Default|GetStaticMesh))
  (if (not (Variables|Default|Getfliped\))
    (Physics|AddImpulse _staticmesh (Math|Vector|MakeVector 0.0 0.0 (Math|Random|RandomFloatinRange 7.5e+02 1e+03)) "None" true)
    (Class|PrimitiveComponent|AddAngularImpulseinDegrees _staticmesh (Math|Vector|MakeVector (Math|Random|RandomFloatinRange 1e+03 1.5e+03) 0.0 0.0) "None" true)
    (Variables|Default|Setfliped\ true)))

(event EventBeginPlay
  (Utilities|FlowControl|Delay 0.2)
  (Input|EnableInput (Game|GetPlayerController 0)))

(event Collision|EventActorBeginOverlap
  (params (OtherActor :type Actor%20Object%20Reference)))

(event EventTick
  (params (DeltaSeconds :type Float%20%28single-precision%29))
  (Utilities|FlowControl|Sequence
    (:then_0
      (if (Class|PrimitiveComponent|IsOverlappingComponent (Variables|Default|Gettail) (Variables|Default|GetPlane))
        (Utilities|FlowControl|DoOnce false :!label _label
          (:Completed
            (bind _asgi_mainmenu (Utilities|Casting|CastToGI_mainmenu (Game|GetGameInstance)))
            (Variables|/Game/GI_mainmenu.GI_mainmenu_C|Setplayer _asgi_mainmenu false)))
        (else
          (goto _label Reset))))
    (:then_1
      (if (Class|PrimitiveComponent|IsOverlappingComponent (Variables|Default|Gethead) (Variables|Default|GetPlane))
        (Utilities|FlowControl|DoOnce false :!label _label_2
          (:Completed
            (bind _asgi_mainmenu_2 (Utilities|Casting|CastToGI_mainmenu (Game|GetGameInstance)))
            (Variables|/Game/GI_mainmenu.GI_mainmenu_C|Setplayer _asgi_mainmenu_2 true)))
        (else
          (goto _label_2 Reset))))))

(fn ConstructionScript)