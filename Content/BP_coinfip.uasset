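; BP_coinfip is an actor that performs a physics-driven coin flip when the A key is pressed.
; Shortly after BeginPlay it enables input from the first player controller.
; Each press applies random upward and X-axis angular impulses to the StaticMesh as velocity changes, ignoring mass.
; A random-yaw rotation node is left unconnected, and no logic reads the landing result.
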(event EventBeginPlay
  (Utilities|FlowControl|Delay 0.2)
  (Input|EnableInput (Game|GetPlayerController 0)))

(event Collision|EventActorBeginOverlap
  (params (OtherActor :type Actor%20Object%20Reference)))

(event EventTick
  (params (DeltaSeconds :type Float%20%28single-precision%29)))

(event Input|KeyboardEvents|A
  (params (Key :type Key%20Structure :default "None"))
  (bind _staticmesh (Variables|Default|GetStaticMesh))
  (:Pressed
    (Physics|AddImpulse _staticmesh (Math|Vector|MakeVector 0.0 0.0 (Math|Random|RandomFloatinRange 7.5e+02 1e+03)) "None" true)
    (Class|PrimitiveComponent|AddAngularImpulseinDegrees _staticmesh (Math|Vector|MakeVector (Math|Random|RandomFloatinRange 1e+03 1.5e+03) 0.0 0.0) "None" true)))

(fn ConstructionScript)